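; Lobby player controller that owns the lobby UI and relays each player's ready state and name.
; It creates the W_Lobby widget when the game state begins and updates it as players join, leave or change readiness.
; Ready changes are manually replicated through every connected controller, then the lobby game mode checks whether everyone is ready.
; The saved profile name is sent to the server, where the game mode applies it.
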(event `OnGameStateBegin`
  (bind _returnvalue (`|CreateWidget` "/Game/UI/Lobby/W_Lobby.W_Lobby_C" self))
  (bind _output_get (set `self.W_Lobby` _returnvalue))
  (`UserWidget.AddToViewport` _output_get 0)
  (`WidgetBlueprintLibrary.SetInputMode_UIOnlyEx` self (`self.W_Lobby`)))

(event `NotifyServerReady`
  (params (Ready :type Boolean))
  (bind _return_value (`/Game/Blueprints/Utility/LIB_BP_Casting.Get Lobby Game Mode`))
  (bind _asps_lobby (cast `/Game/Blueprints/Lobby/PS_Lobby` (`self.PlayerState`) :!pure true))
  ;[1 1 1] Set/ManuallyReplicate Ready
  (bind _output_get (set `/Game/Blueprints/Lobby/PS_Lobby.Ready` Ready _asps_lobby))
  (bind _values (`BlueprintMapLibrary.Map_Values` (`/Game/Blueprints/Lobby/GM_Lobby.ConnectedPlayers` _return_value)))
  (`self.ReplicateReady` _values (`PlayerState.PlayerId` _asps_lobby) _output_get)
  (`/Game/Blueprints/Lobby/GM_Lobby.CheckIfEveryoneReady` _return_value))

(event `ReplicateReady`
  (params (ID :type Integer) (Ready :type Boolean))
  ;[1 1 1] Set/ManuallyReplicate Ready
  (bind _player_state (`/Game/Blueprints/Utility/LIB_BP_General.Get Player State` ID))
  (set `/Game/Blueprints/Lobby/PS_Lobby.Ready` Ready (cast `/Game/Blueprints/Lobby/PS_Lobby` _player_state :!pure true))
  (`/Game/UI/Lobby/W_Lobby.UpdatePlayer` (`self.W_Lobby`) ID))

(event `OnPlayerStateAdded`
  (params (PS_Lobby :type "/Game/Blueprints/Lobby/PS_Lobby Object Reference"))
  (`/Game/UI/Lobby/W_Lobby.AddPlayer` (`self.W_Lobby`) PS_Lobby))

(event `OnPlayerLeave`
  (params (ID :type Integer))
  (bind _w_lobby (`self.W_Lobby`))
  (`/Engine/EditorBlueprintResources/StandardMacros.IsValid` _w_lobby
    (:`Is Valid`
      (`/Game/UI/Lobby/W_Lobby.RemovePlayer` _w_lobby ID))))

(event `self.ReceiveDestroyed`
  (bind _w_lobby (`self.W_Lobby`))
  (`/Engine/EditorBlueprintResources/StandardMacros.IsValid` _w_lobby
    (:`Is Valid`
      (`Widget.RemoveFromParent` _w_lobby))))

(event `GetDesiredName`
  (bind _return_value (`/Game/Blueprints/Utility/LIB_BP_Casting.Get Project Game Instance`))
  (bind _returnvalue (`/Game/Blueprints/Utility/LIB_M_General.Find Save Game By Slot` (`/Game/Blueprints/GI.SAVE_SLOT_PROFILE` _return_value) (`/Game/Blueprints/GI.SAVE_SLOT_ID` _return_value))
    (:`then`
      (bind _assg_player_profile (cast `/Game/Blueprints/SG_PlayerProfile` _returnvalue))
      (`self.SetName(Server)` (`/Game/Blueprints/SG_PlayerProfile.Name` _assg_player_profile)))))

(event `SetName(Server)`
  (params (Name :type String))
  (`GameModeBase.ChangeName` (`GameplayStatics.GetGameMode`) self Name true))

(fn `UserConstructionScript`)