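; AO_Raise is a tile effect actor that changes terrain altitude when its play ends.
; On EndPlay it runs the parent logic, then plays the TerrainBump sound at its location.
; It applies an altitude change of Distance to its own Position, then to each tile in TilesUnderEffect.
; The construction script only calls the parent.
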(event `self.ReceiveEndPlay`
  (params (EndPlayReason :type "EEndPlayReason Enum" :default "Destroyed"))
  (`parent.ReceiveEndPlay` EndPlayReason)
  (`GameplayStatics.PlaySoundAtLocation` "/Game/Sounds/TerrainBump.TerrainBump" (`self.K2_GetActorLocation`))
  (`self.ApplyEffect_AltitudeChange` (`self.Position`) (`self.Distance`))
  (for _array_element (`self.TilesUnderEffect`)
    (`self.ApplyEffect_AltitudeChange` _array_element (`self.Distance`))))

(fn `UserConstructionScript`
  (`parent.UserConstructionScript`))