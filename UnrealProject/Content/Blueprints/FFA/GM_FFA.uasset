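; Game mode for FFA that manages connected players, team assignment and the collector placement phase.
; Login and controller swaps pass map settings to the controller, register it by PlayerId and set an alternating TeamId from the player count, which FindPlayerStart uses as a PlayerStart index.
; Logout sends a "Left Game" feed entry to remaining players.
; CheckIfAllCollectorsPlaced calls CollectorPhaseOver on all controllers once every player is ready.
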(event `self.K2_OnSwapPlayerControllers`
  (params (OldPC :type "PlayerController Object Reference") (NewPC :type "PlayerController Object Reference"))
  (bind _aspc_ffa (cast `/Game/Blueprints/FFA/PC_FFA` NewPC :!pure true))
  (set `/Game/Blueprints/FFA/PC_FFA.MAP` (`/Game/Blueprints/GI.MapSettings` (`/Game/Blueprints/Utility/LIB_BP_Casting.Get Project Game Instance`)) _aspc_ffa)
  (`BlueprintMapLibrary.Map_Add` (`self.ConnectedPlayers`) (`PlayerState.PlayerId` (`Controller.PlayerState` _aspc_ffa)) _aspc_ffa)
  (set `/Game/Blueprints/FFA/PS_FFA.TeamId` (mod (`BlueprintMapLibrary.Map_Length` (`self.ConnectedPlayers`)) 2) (cast `/Game/Blueprints/FFA/PS_FFA` (`Controller.PlayerState` _aspc_ffa) :!pure true))
  (`KismetSystemLibrary.PrintString` (`KismetStringLibrary.Concat_StrStr` "SWAPPING PC TO: " (`KismetSystemLibrary.GetClassDisplayName` (`GameplayStatics.GetObjectClass` NewPC))) true true (struct :`R` 1.0 :`G` 0.065432 :`A` 1.0) 20.0))

(event `self.K2_PostLogin`
  (params (NewPlayer :type "PlayerController Object Reference"))
  (bind _aspc_ffa (cast `/Game/Blueprints/FFA/PC_FFA` NewPlayer :!pure true))
  (bind _playerstate (`Controller.PlayerState` _aspc_ffa))
  (set `/Game/Blueprints/FFA/PC_FFA.MAP` (`/Game/Blueprints/GI.MapSettings` (`/Game/Blueprints/Utility/LIB_BP_Casting.Get Project Game Instance`)) _aspc_ffa)
  (`BlueprintMapLibrary.Map_Add` (`self.ConnectedPlayers`) (`PlayerState.PlayerId` _playerstate) _aspc_ffa)
  (bind _output_get (set `/Game/Blueprints/FFA/PS_FFA.TeamId` (mod (`BlueprintMapLibrary.Map_Length` (`self.ConnectedPlayers`)) 2) (cast `/Game/Blueprints/FFA/PS_FFA` _playerstate :!pure true)))
  (`KismetSystemLibrary.PrintString` (`KismetStringLibrary.Concat_StrStr` "Login PC" " " (`KismetStringLibrary.Conv_IntToString` _output_get)) true true (struct :`R` 0.005958 :`G` 1.0 :`A` 1.0) 20.0))

(event `self.K2_OnLogout`
  (params (ExitingController :type "Controller Object Reference"))
  (bind _playerstate (`Controller.PlayerState` ExitingController))
  (bind _playerid (`PlayerState.PlayerId` _playerstate))
  (`BlueprintMapLibrary.Map_Remove` (`self.ConnectedPlayers`) _playerid)
  (bind _values (`BlueprintMapLibrary.Map_Values` (`self.ConnectedPlayers`)))
  (`/Game/Blueprints/FFA/PC_FFA.RecieveFeedEntry` _values (make `/Game/UI/NotificationFeed/S_GameMessage` "NewEnumerator3" _playerid (`|FormatText` "{Player} Left Game" (`KismetTextLibrary.Conv_StringToText` (`PlayerState.PlayerName` _playerstate))))))

(event `self.ReceiveBeginPlay`
  (`KismetSystemLibrary.PrintString` "GM BP" true true (struct :`R` 1.0 :`B` 0.026084 :`A` 1.0) 20.0))

(fn `CheckIfAllCollectorsPlaced`
  (locals (ReadyCount :type Integer))
  (bind _playerarray (`GameStateBase.PlayerArray` (`GameplayStatics.GetGameState`)))
  (for _array_element _playerarray
    (bind _asps_ffa (cast `/Game/Blueprints/FFA/PS_FFA` _array_element))
    (`/Game/Blueprints/Utility/LIB_BP_General.+=(Int)` (`local.ReadyCount`) (`KismetMathLibrary.Conv_BoolToInt` (`/Game/Blueprints/FFA/PS_FFA.CollectorPlaced` _asps_ffa))))
  (if (== (`KismetArrayLibrary.Array_Length` _playerarray) (`local.ReadyCount`))
    (bind _values (`BlueprintMapLibrary.Map_Values` (`self.ConnectedPlayers`)))
    (for _array_element_2 _values
      (`/Game/Blueprints/FFA/PC_FFA.CollectorPhaseOver` _array_element_2))))

(fn `ChoosePlayerStart`
  (params (Player :type "Controller Object Reference"))
  (returns (ReturnValue :type "Actor Object Reference"))
  (return null))

(fn `FindPlayerStart`
  (params (Player :type "Controller Object Reference") (IncomingName :type String))
  (returns (ReturnValue :type "Actor Object Reference"))
  (bind _teamid (`/Game/Blueprints/FFA/PS_FFA.TeamId` (cast `/Game/Blueprints/FFA/PS_FFA` (`Controller.PlayerState` Player) :!pure true)))
  (bind _outactors (`GameplayStatics.GetAllActorsOfClass` "/Script/Engine.PlayerStart"))
  (`KismetSystemLibrary.PrintString` (`KismetStringLibrary.Conv_IntToString` _teamid) true true (struct :`A` 1.0) 10.0)
  (return (`|GetArrayItem` _outactors _teamid)))

(fn `UserConstructionScript`)