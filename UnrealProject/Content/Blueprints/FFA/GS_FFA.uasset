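; Game State for the FFA mode that spawns the world, tracks creature counts per team and ends the match.
; On authority it polls until the first FFA player controller is valid, then spawns the WorldGenerator.
; Non-dedicated instances time the match from that controller's map setting, then EndGame broadcasts the team with most creatures and pauses.
; Helpers supply team colors, population percentages and materials, with creature materials chosen by respiration type.
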(event `self.ReceiveBeginPlay`
  (bind _return_value (`/Game/Blueprints/Utility/LIB_BP_Casting.Get FFA Player Controller` 0))
  (bind _map_time (break `/Game/S_MapSettings` (`/Game/Blueprints/FFA/PC_FFA.MAP` _return_value)))
  (`/Engine/EditorBlueprintResources/ActorMacros.Switch Has Authority`
    (:`Authority`
      (`/Engine/EditorBlueprintResources/StandardMacros.IsValid` (`/Game/Blueprints/Utility/LIB_BP_Casting.Get FFA Player Controller` 0) :!label _label
        (:`Is Valid`
          (`self.SpawnWorld`))
        (:`Is Not Valid`
          (`KismetSystemLibrary.Delay` 0.2)
          (goto _label))))
    (:`Remote`
      _))
  (`KismetSystemLibrary.PrintString` "GS STARTING" true true (struct :`R` 0.890561 :`B` 1.0 :`A` 1.0) 20.0)
  (if (`KismetSystemLibrary.IsDedicatedServer`)
    (`KismetSystemLibrary.PrintString` "IAM A DEDICATED SERVER" true true (struct :`R` 0.890561 :`B` 1.0 :`A` 1.0) 20.0)
    (else
      (`/Engine/EditorBlueprintResources/StandardMacros.IsValid` _return_value :!label _label_2
        (:`Is Valid`
          (`KismetSystemLibrary.K2_SetTimerDelegate` (delegate `End Game`) (`KismetMathLibrary.Conv_IntToDouble` (* _map_time 60))))
        (:`Is Not Valid`
          (`KismetSystemLibrary.Delay` 0.2)
          (goto _label_2))))))

(event `End Game`
  (`self.OnEndGame` (`KismetMathLibrary.MaxOfIntArray` (`self.TeamCreatureCount`)))
  (`GameplayStatics.SetGamePaused` true))

(fn `DecrementTeamCount`
  (params (TeamId :type Integer))
  (`/Engine/EditorBlueprintResources/StandardMacros.DecrementInt` (`|GetArrayItem` (`self.TeamCreatureCount`) TeamId)
    (:`  `
      (return))))

(fn `GetTeamCollectorMat`
  (params (TeamId :type Integer))
  (returns (Material :type "MaterialInstanceConstant Object Reference"))
  (return (`|GetArrayItem` (`self.TeamCollectorMaterials`) TeamId)))

(fn `GetTeamColor`
  (params (TeamId :type Integer))
  (returns (Output :type "LinearColor Structure (by ref)"))
  (return (`|GetArrayItem` (`self.TeamColors`) TeamId)))

(fn `GetTeamCreatureMat`
  (params (TeamId :type Integer) (Respiration :type "/Game/RespirationType Enum" :default "NewEnumerator0"))
  (returns (Material :type "MaterialInstanceConstant Object Reference"))
  (switch `/Game/RespirationType` Respiration
    (:`NewEnumerator0`
      (return (`|GetArrayItem` (`self.TeamCreatureMaterials(Land)`) TeamId)))
    (:`NewEnumerator1`
      (return (`|GetArrayItem` (`self.TeamCreatureMaterials(Water)`) TeamId)))
    (:`NewEnumerator2`
      (return (`|GetArrayItem` (`self.TeamCreatureMaterials(Amphibian)`) TeamId)))))

(fn `GetTeamPercent`
  (params (TeamId :type Integer))
  (returns (ReturnValue :type Integer))
  (return (/ (* (`|GetArrayItem` (`self.TeamCreatureCount`) TeamId) 100) (`KismetArrayLibrary.Array_Length` (`/Game/WorldGenerator.Creature` (`self.WorldGen`))))))

(fn `IncrementTeamCount`
  (params (TeamId :type Integer))
  (`/Engine/EditorBlueprintResources/StandardMacros.IncrementInt` (`|GetArrayItem` (`self.TeamCreatureCount`) TeamId)
    (:`  `
      (return))))

(fn `SpawnWorld`
  (bind _returnvalue (`|SpawnActorFromClass` "/Game/WorldGenerator.WorldGenerator_C" (`KismetMathLibrary.MakeTransform` (0.0 0.0 0.0)) "AlwaysSpawn" "OverrideRootScale" null (struct) null))
  (set `self.WorldGen` _returnvalue))

(fn `UserConstructionScript`
  (`KismetSystemLibrary.PrintString` "GS Construct"))