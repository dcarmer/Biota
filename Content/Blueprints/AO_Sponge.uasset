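; AO_Sponge is an action object that soaks up liquids on the world grid.
; On BeginPlay it scans the tiles under its effect and destroys any water or goo action objects occupying them in the game state's WorldGen.
; Each tick it applies a food change to every tile under its effect, scaled by delta time and its food-per-second rate.
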(event `self.ReceiveBeginPlay`
  (`parent.ReceiveBeginPlay`)
  (for _array_element (`self.TilesUnderEffect`)
    (bind _output (`|GetArrayItem` (`/Game/WorldGenerator.ActionObjects` (`/Game/Blueprints/FFA/GS_FFA.WorldGen` (`/Game/Blueprints/Utility/LIB_BP_Casting.Get FFA Game State`))) _array_element))
    (`/Engine/EditorBlueprintResources/StandardMacros.IsValid` _output
      (:`Is Valid`
        (bind _returnvalue (`GameplayStatics.GetObjectClass` _output))
        (if (or (`KismetMathLibrary.ClassIsChildOf` _returnvalue "/Game/Blueprints/AO_Water.AO_Water_C") (`KismetMathLibrary.ClassIsChildOf` _returnvalue "/Game/Blueprints/AO_Goo.AO_Goo_C"))
          (`self.K2_DestroyActor` _output))))))

(event `self.ReceiveTick`
  (params (DeltaSeconds :type "Float (single-precision)"))
  (for _array_element (`self.TilesUnderEffect`)
    (`self.ApplyEffect_FoodChange` _array_element (* DeltaSeconds (`self.Food per Sec`)))))

(fn `UserConstructionScript`
  (`parent.UserConstructionScript`))