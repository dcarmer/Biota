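; AO_Water is a water object that changes the gather bonus of the tiles under its effect while it is in play.
; On BeginPlay, after the parent logic, it applies GrowthBonus to each position in TilesUnderEffect.
; On EndPlay it applies the negated GrowthBonus over the same array to undo the change.
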(event `self.ReceiveBeginPlay`
  (`parent.ReceiveBeginPlay`)
  (for _array_element (`self.TilesUnderEffect`)
    (`self.ApplyEffect_GatherBonusChange` _array_element (`self.GrowthBonus`))))

(event `self.ReceiveEndPlay`
  (params (EndPlayReason :type "EEndPlayReason Enum" :default "Destroyed"))
  (`parent.ReceiveEndPlay` EndPlayReason)
  (for _array_element (`self.TilesUnderEffect`)
    (`self.ApplyEffect_GatherBonusChange` _array_element (* (`self.GrowthBonus`) -1.0))))

(fn `UserConstructionScript`
  (`parent.UserConstructionScript`))