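; TNT action object that explodes when it ends play, whatever the end-play reason.
; For each tile in TilesUnderEffect, it applies Damage as a health change, then destroys any valid action object at that tile in the FFA game state's WorldGen.
; Destroying another TNT this way fires its own EndPlay, so blasts can chain.
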(event `self.ReceiveEndPlay`
  (params (EndPlayReason :type "EEndPlayReason Enum" :default "Destroyed"))
  (`parent.ReceiveEndPlay` EndPlayReason)
  (for _array_element (`self.TilesUnderEffect`)
    (`self.ApplyEffect_HealthChange` _array_element (`self.Damage`))
    (bind _output (`|GetArrayItem` (`/Game/WorldGenerator.ActionObjects` (`/Game/Blueprints/FFA/GS_FFA.WorldGen` (`/Game/Blueprints/Utility/LIB_BP_Casting.Get FFA Game State`))) _array_element))
    (`/Engine/EditorBlueprintResources/StandardMacros.IsValid` _output
      (:`Is Valid`
        (`self.K2_DestroyActor` _output)))))

(fn `UserConstructionScript`
  (`parent.UserConstructionScript`))