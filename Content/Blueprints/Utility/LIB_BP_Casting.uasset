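; Blueprint function library of typed getters for the project's Lobby and FFA framework classes and its Game Instance.
; Each function casts the engine's game mode, game state, player controller or game instance to the project class, with controllers found by player index or a target's owning player.
; Failed casts print a long-lasting red error, with index or target name for controllers, except the Lobby Game State getter, which casts silently.
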(fn `Get FFA Game Mode`
  (returns (`Return Value` :type "/Game/Blueprints/FFA/GM_FFA Object Reference"))
  (bind _asgm_ffa (cast `/Game/Blueprints/FFA/GM_FFA` (`GameplayStatics.GetGameMode` null))
    (:`then`
      (return _asgm_ffa))
    (:`CastFailed`
      (`KismetSystemLibrary.PrintString` null "CAST FAILED: GM_FFA" true true (struct :`R` 1.0 :`B` 0.012675 :`A` 1.0) 20.0))))

(fn `Get FFA Player Controller`
  (params (PlayerIndex :type Integer))
  (returns (`Return Value` :type "/Game/Blueprints/FFA/PC_FFA Object Reference"))
  (bind _aspc_ffa (cast `/Game/Blueprints/FFA/PC_FFA` (`GameplayStatics.GetPlayerController` null PlayerIndex))
    (:`then`
      (return _aspc_ffa))
    (:`CastFailed`
      (`KismetSystemLibrary.PrintString` null (`KismetStringLibrary.Concat_StrStr` "CAST FAILED: PC_FFA " (`KismetStringLibrary.Conv_IntToString` PlayerIndex)) true true (struct :`R` 1.0 :`B` 0.012675 :`A` 1.0) 20.0))))

(fn `Get Lobby Game Mode`
  (returns (`Return Value` :type "/Game/Blueprints/Lobby/GM_Lobby Object Reference"))
  (bind _asgm_lobby (cast `/Game/Blueprints/Lobby/GM_Lobby` (`GameplayStatics.GetGameMode` null))
    (:`then`
      (return _asgm_lobby))
    (:`CastFailed`
      (`KismetSystemLibrary.PrintString` null "CAST FAILED: GM_Lobby" true true (struct :`R` 1.0 :`B` 0.012675 :`A` 1.0) 20.0))))

(fn `Get Lobby Game State`
  (returns (`Return Value` :type "/Game/Blueprints/Lobby/GS_Lobby Object Reference"))
  (return (cast `/Game/Blueprints/Lobby/GS_Lobby` (`GameplayStatics.GetGameState` null) :!pure true)))

(fn `Get Lobby Player Controller`
  (params (PlayerIndex :type Integer))
  (returns (`Return Value` :type "/Game/Blueprints/Lobby/PC_Lobby Object Reference"))
  (bind _aspc_lobby (cast `/Game/Blueprints/Lobby/PC_Lobby` (`GameplayStatics.GetPlayerController` null PlayerIndex))
    (:`then`
      (return _aspc_lobby))
    (:`CastFailed`
      (`KismetSystemLibrary.PrintString` null (`KismetStringLibrary.Concat_StrStr` "CAST FAILED: PC_Lobby " (`KismetStringLibrary.Conv_IntToString` PlayerIndex)) true true (struct :`R` 1.0 :`B` 0.012675 :`A` 1.0) 20.0))))

(fn `Get Owning FFA Player`
  (params (Target :type "UserWidget Object Reference"))
  (returns (`Return Value` :type "/Game/Blueprints/FFA/PC_FFA Object Reference"))
  (bind _aspc_ffa (cast `/Game/Blueprints/FFA/PC_FFA` (`UserWidget.GetOwningPlayer` Target))
    (:`then`
      (return _aspc_ffa))
    (:`CastFailed`
      (`KismetSystemLibrary.PrintString` null (`KismetStringLibrary.Concat_StrStr` "CAST FAILED: PC_FFA" (`KismetSystemLibrary.GetDisplayName` Target)) true true (struct :`R` 1.0 :`B` 0.012675 :`A` 1.0) 20.0))))

(fn `Get Owning Lobby Player`
  (params (Target :type "UserWidget Object Reference"))
  (returns (`Return Value` :type "/Game/Blueprints/Lobby/PC_Lobby Object Reference"))
  (bind _aspc_lobby (cast `/Game/Blueprints/Lobby/PC_Lobby` (`UserWidget.GetOwningPlayer` Target))
    (:`then`
      (return _aspc_lobby))
    (:`CastFailed`
      (`KismetSystemLibrary.PrintString` null (`KismetStringLibrary.Concat_StrStr` "CAST FAILED: PC_Lobby " (`KismetSystemLibrary.GetDisplayName` Target)) true true (struct :`R` 1.0 :`B` 0.012675 :`A` 1.0) 20.0))))

(fn `Get Project Game Instance`
  (returns (`Return Value` :type "/Game/Blueprints/GI Object Reference"))
  (bind _asgi (cast `/Game/Blueprints/GI` (`GameplayStatics.GetGameInstance` null))
    (:`then`
      (return _asgi))
    (:`CastFailed`
      (`KismetSystemLibrary.PrintString` null "CAST FAILED: GI " true true (struct :`R` 1.0 :`B` 0.012675 :`A` 1.0) 20.0))))