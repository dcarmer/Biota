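; Goo hazard object that covers the valid world tiles within RADIUS of its grid Position and displays a lifespan timer.
; On BeginPlay it asks the FFA game state's WorldGen for those tiles and adds an instanced static mesh at each.
; It also seeds the billboard TimerBar widget with InitialLifeSpan.
; GetValidInRange is a local ring-by-ring neighbor search that BeginPlay does not use.
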(event `self.ReceiveBeginPlay`
  (bind _initiallifespan (`self.InitialLifeSpan`))
  (bind _worldgen (`/Game/Blueprints/FFA/GS_FFA.WorldGen` (`/Game/Blueprints/Utility/LIB_BP_Casting.Get FFA Game State`)))
  (bind _result (`/Game/WorldGenerator.GetValidNeighborsInRange` _worldgen (`self.Position`) (`self.RADIUS`)))
  (for _array_element _result
    (bind _transform (`/Game/WorldGenerator.GetTileTransform` _worldgen _array_element))
    (`InstancedStaticMeshComponent.AddInstanceWorldSpace` (`self.InstancedStaticMesh`) (`KismetMathLibrary.MakeTransform` (.location _transform) (struct) (`SceneComponent.K2_GetComponentScale` (`self.InstancedStaticMesh`)))))
  (bind _astimer_bar (cast `/Game/UI/TimerBar` (`WidgetComponent.GetUserWidgetObject` (`self.WidgetBillboard`))))
  (set `/Game/UI/TimerBar.Initial` _initiallifespan _astimer_bar)
  (set `/Game/UI/TimerBar.Current` _initiallifespan _astimer_bar))

(fn `GetValidInRange`
  (returns (Result :type "Array of Integer"))
  (locals (WorkingSet :type "Set of Integer") (PendingSet :type "Set of Integer") (TotalSet :type "Set of Integer"))
  (bind _totalset (`local.TotalSet`))
  (`BlueprintSetLibrary.Set_Add` (`local.WorkingSet`) (`self.Position`))
  (for _ (range 1 (+ (`self.RADIUS`) 1))
    (bind _result (`BlueprintSetLibrary.Set_ToArray` (`local.WorkingSet`)))
    (for _array_element _result
      (bind _neighbors (`/Game/WorldGenerator.GetValidNeighbors` (`/Game/Blueprints/FFA/GS_FFA.WorldGen` (`/Game/Blueprints/Utility/LIB_BP_Casting.Get FFA Game State`)) _array_element))
      (`BlueprintSetLibrary.Set_AddItems` (`local.PendingSet`) _neighbors)
      (`BlueprintSetLibrary.Set_AddItems` (`local.TotalSet`) _neighbors))
    (set `local.WorkingSet` (`local.PendingSet`))
    (`BlueprintSetLibrary.Set_Clear` (`local.PendingSet`)))
  (`BlueprintSetLibrary.Set_Remove` _totalset (`self.Position`))
  (bind _result_2 (`BlueprintSetLibrary.Set_ToArray` _totalset))
  (return _result_2))

(fn `UserConstructionScript`)