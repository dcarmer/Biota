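; Lobby game mode that tracks connected players and starts the game once everyone is ready.
; On login it gives each PlayerState a random color, maps PlayerId to controller, and notifies a listen-server host of remote players.
; On logout it unmaps the player and tells the remaining controllers.
; CheckIfEveryoneReady compares ready count to PlayerArray, starting or cancelling a delayed timer that calls the game instance's StartGame.
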(event `self.K2_PostLogin`
  (params (NewPlayer :type "PlayerController Object Reference"))
  (bind _aspc_lobby (cast `/Game/Blueprints/Lobby/PC_Lobby` NewPlayer :!pure true))
  (bind _asps_lobby (cast `/Game/Blueprints/Lobby/PS_Lobby` (`Controller.PlayerState` _aspc_lobby) :!pure true))
  (set `/Game/Blueprints/Lobby/PS_Lobby.Color` (make `LinearColor` (`KismetMathLibrary.RandomFloat`) (`KismetMathLibrary.RandomFloat`) (`KismetMathLibrary.RandomFloat`) 1.0) _asps_lobby)
  (`BlueprintMapLibrary.Map_Add` (`self.ConnectedPlayers`) (`PlayerState.PlayerId` _asps_lobby) _aspc_lobby)
  ;[1 1 1] BC: On Server side, this is the first time remote Player States have been initialized
  (if (not (or (`KismetSystemLibrary.IsDedicatedServer`) (`Controller.IsLocalPlayerController` _aspc_lobby)))
    (`/Game/Blueprints/Lobby/PC_Lobby.OnPlayerStateAdded` (`/Game/Blueprints/Utility/LIB_BP_Casting.Get Lobby Player Controller` 0) _asps_lobby)))

(event `self.K2_OnLogout`
  (params (ExitingController :type "Controller Object Reference"))
  (bind _playerid (`PlayerState.PlayerId` (`Controller.PlayerState` ExitingController)))
  (`BlueprintMapLibrary.Map_Remove` (`self.ConnectedPlayers`) _playerid)
  ;[1 1 1] Let the remaining players know someone left
  (bind _values (`BlueprintMapLibrary.Map_Values` (`self.ConnectedPlayers`)))
  (`/Game/Blueprints/Lobby/PC_Lobby.OnPlayerLeave` _values _playerid))

(event `EnterStartGame`
  (bind _returnvalue (`KismetSystemLibrary.K2_SetTimerDelegate` (delegate `StartGame`) (`/Game/Blueprints/Lobby/GS_Lobby.START_DELAY` (`/Game/Blueprints/Utility/LIB_BP_Casting.Get Lobby Game State`)))))

(event `CancelStartGame`
  (`KismetSystemLibrary.K2_ClearAndInvalidateTimerHandle` (stale `EnterStartGame` _returnvalue)))

(event `StartGame`
  (`KismetSystemLibrary.PrintString` "STARTING GAME" true true (struct :`R` 1.0 :`G` 0.018362 :`A` 1.0) 20.0)
  (`/Game/Blueprints/GI.StartGame` (`/Game/Blueprints/Utility/LIB_BP_Casting.Get Project Game Instance`)))

(event `self.K2_OnSwapPlayerControllers`
  (params (OldPC :type "PlayerController Object Reference") (NewPC :type "PlayerController Object Reference"))
  (`KismetSystemLibrary.PrintString` "SWAP: LOBBY" true true (struct :`G` 0.66 :`B` 1.0 :`A` 1.0) 20.0))

(event `self.HandleStartingNewPlayer`
  (params (NewPlayer :type "PlayerController Object Reference"))
  (`KismetSystemLibrary.PrintString` (`KismetStringLibrary.Concat_StrStr` "OPTIONS: " (`self.OptionsString`)) true true (struct :`G` 1.0 :`B` 0.044676 :`A` 1.0) 20.0))

(fn `CheckIfEveryoneReady`
  (locals (ReadyCount :type Integer))
  (bind _playerarray (`GameStateBase.PlayerArray` (`GameplayStatics.GetGameState`)))
  (for _array_element _playerarray
    (`/Game/Blueprints/Utility/LIB_BP_General.+=(Int)` (`local.ReadyCount`) (`KismetMathLibrary.Conv_BoolToInt` (`/Game/Blueprints/Lobby/PS_Lobby.Ready` (cast `/Game/Blueprints/Lobby/PS_Lobby` _array_element :!pure true)))))
  (if (== (`KismetArrayLibrary.Array_Length` _playerarray) (`local.ReadyCount`))
    (`self.EnterStartGame`)
    (else
      (`self.CancelStartGame`))))

(fn `UserConstructionScript`)