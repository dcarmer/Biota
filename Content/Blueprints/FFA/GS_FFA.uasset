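; Game State for the FFA mode that tracks teams and ends the match on a timer.
; Teams get a random color and a creature count, with percentages measured against the creature list of the WorldGenerator found in the construction script.
; On non-dedicated instances, BeginPlay notifies the local PC_FFA and starts the game-over timer.
; When it fires, the team with the most creatures is passed to CallOnEndGame and the game pauses.
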(event `self.ReceiveBeginPlay`
  (`KismetSystemLibrary.PrintString` "GS STARTING" true true (struct :`R` 0.890561 :`B` 1.0 :`A` 1.0) 20.0)
  (if (`KismetSystemLibrary.IsDedicatedServer`)
    (`KismetSystemLibrary.PrintString` "IAM A DEDICATED SERVER" true true (struct :`R` 0.890561 :`B` 1.0 :`A` 1.0) 20.0)
    (else
      (bind _aspc_ffa (cast `/Game/Blueprints/FFA/PC_FFA` (`GameplayStatics.GetPlayerController` 0))
        (:`then`
          (`/Game/Blueprints/FFA/PC_FFA.OnGameStateBegin` _aspc_ffa)
          (`KismetSystemLibrary.K2_SetTimerDelegate` (delegate `End Game`) (* (`self.GameOverAt(min)`) 60.0)))
        (:`CastFailed`
          (`KismetSystemLibrary.PrintString` "PC NOT A FFA" true true (struct :`R` 1.0 :`B` 0.012675 :`A` 1.0) 20.0))))))

(event `End Game`
  (`self.OnEndGame` (`KismetMathLibrary.MaxOfIntArray` (`self.TeamCreatureCount`)))
  (`GameplayStatics.SetGamePaused` true))

(fn `GetTeamColor`
  (params (TeamId :type Integer))
  (returns (Output :type "LinearColor Structure (by ref)"))
  (return (`|GetArrayItem` (`self.TeamColors`) TeamId)))

(fn `GetTeamPercent`
  (params (TeamId :type Integer))
  (returns (ReturnValue :type Integer))
  (return (/ (* (`|GetArrayItem` (`self.TeamCreatureCount`) TeamId) 100) (`KismetArrayLibrary.Array_Length` (`/Game/WorldGenerator.Creature` (`self.WorldGen`))))))

(fn `MakeNewTeam`
  (returns (TeamId :type Integer))
  (bind _returnvalue (`KismetArrayLibrary.Array_Add` (`self.TeamColors`) (make `LinearColor` (`KismetMathLibrary.RandomFloat`) (`KismetMathLibrary.RandomFloat`) (`KismetMathLibrary.RandomFloat`) 1.0)))
  (`KismetArrayLibrary.Array_Add` (`self.TeamCreatureCount`))
  (return _returnvalue))

(fn `UserConstructionScript`
  (bind _outactors (`GameplayStatics.GetAllActorsOfClass` "/Game/WorldGenerator.WorldGenerator_C"))
  (set `self.WorldGen` (`|GetArrayItem` _outactors)))