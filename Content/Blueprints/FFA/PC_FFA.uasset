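; Player controller for FFA mode that sets up the HUD and minimap render target once both BeginPlay and game-state start have fired.
; Input drives pause, player list and chat; feed entries relay through the GameMode's ConnectedPlayers, with team chat currently reaching everyone.
; Clicks convert the hit hex instance to a WorldGenerator index: left spawns a creature, right lowers altitude via server-to-all-clients relay.
; EndPlay destroys the session.
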(event `self.ReceiveBeginPlay`
  (`KismetSystemLibrary.PrintString` "PCCCC STARTING" true true (struct :`R` 0.890561 :`B` 1.0 :`A` 1.0) 20.0)
  (`/Game/Blueprints/Utility/LIB_M_General.AND Gate` :!label _label
    (:`C`
      (bind _returnvalue (`KismetRenderingLibrary.CreateRenderTarget2D` 256))
      (set `SceneCaptureComponent2D.TextureTarget` _returnvalue (`self.MiniMapCapture`))
      (bind _returnvalue_2 (`|CreateWidget` "/Game/UI/W_HUD.W_HUD_C" self))
      (bind _output_get (set `self.GameHUD` _returnvalue_2))
      (`UserWidget.AddToViewport` _output_get 0)
      (`WidgetBlueprintLibrary.SetInputMode_GameAndUIEx` self null "DoNotLock" false))))

(event `OnGameStateBegin`
  (`KismetSystemLibrary.PrintString` "GS-PC STARTING" true true (struct :`R` 0.890561 :`B` 1.0 :`A` 1.0) 20.0)
  (goto _label :!via `B`))

(event `InputAction|Pause`
  (params (Key :type "Key Structure"))
  (:`Pressed`
    (`/Game/UI/W_HUD.TogglePauseMenu` (`self.GameHUD`))))

(event `InputAction|ShowConnectedPlayers`
  (params (Key :type "Key Structure"))
  (bind _gamehud (`self.GameHUD`))
  (:`Pressed`
    (`/Game/UI/W_HUD.ShowPlayerList` _gamehud))
  (:`Released`
    (`/Game/UI/W_HUD.HidePlayerList` _gamehud)))

(event `InputAction|Chat`
  (params (Key :type "Key Structure"))
  (:`Pressed`
    (`/Game/UI/NotificationFeed/W_NotificationFeed.FocusChat` (`/Game/UI/W_HUD.W_LobbyFeed` (`self.GameHUD`)))))

(event `OnPlayerStateBegin`
  (params (PlayerState :type "/Game/Blueprints/FFA/PS_FFA Object Reference"))
  (`self.RecieveFeedEntry` (make `/Game/UI/NotificationFeed/S_GameMessage` "NewEnumerator3" (`PlayerState.PlayerId` PlayerState) (`|FormatText` "{Player} Joined Game" (`KismetTextLibrary.Conv_StringToText` (`PlayerState.PlayerName` PlayerState))))))

(event `RecieveFeedEntry`
  (params (Entry :type "/Game/UI/NotificationFeed/S_GameMessage Structure"))
  ;[1 1 1] Server-Client Chat Handling
  (`/Game/UI/NotificationFeed/W_NotificationFeed.LogToFeed` (`/Game/UI/W_HUD.W_LobbyFeed` (`self.GameHUD`)) Entry false))

(event `SendChat ToAll`
  (params (Entry :type "/Game/UI/NotificationFeed/S_GameMessage Structure"))
  ;[1 1 1] Server-Client Chat Handling
  (bind _values (`BlueprintMapLibrary.Map_Values` (`/Game/Blueprints/FFA/GM_FFA.ConnectedPlayers` (`/Game/Blueprints/Utility/LIB_BP_Casting.Get FFA Game Mode`))))
  (`self.RecieveFeedEntry` _values Entry))

(event `SendChat ToTeam`
  (params (Entry :type "/Game/UI/NotificationFeed/S_GameMessage Structure"))
  ;[1 1 1] Server-Client Chat Handling
  (bind _values (`BlueprintMapLibrary.Map_Values` (`/Game/Blueprints/FFA/GM_FFA.ConnectedPlayers` (`/Game/Blueprints/Utility/LIB_BP_Casting.Get FFA Game Mode`))))
  (`self.RecieveFeedEntry` _values Entry))

(event `SendChat ToPlayer`
  (params (PlayerID :type Integer) (Entry :type "/Game/UI/NotificationFeed/S_GameMessage Structure"))
  (bind (_value _returnvalue) (`BlueprintMapLibrary.Map_Find` (`/Game/Blueprints/FFA/GM_FFA.ConnectedPlayers` (`/Game/Blueprints/Utility/LIB_BP_Casting.Get FFA Game Mode`)) PlayerID))
  ;[1 1 1] Server-Client Chat Handling
  (if _returnvalue
    (`self.RecieveFeedEntry` _value Entry)))

(event `self.ReceiveEndPlay`
  (params (EndPlayReason :type "EEndPlayReason Enum" :default "Destroyed"))
  (`DestroySessionCallbackProxy.DestroySession` self
    (:`OnSuccess`
      (`KismetSystemLibrary.PrintString` (`KismetStringLibrary.Concat_StrStr` "END PLAY REASON: " (`|GetEnumeratorNameAsString` EndPlayReason) " SESSION DESTROYED") true true (struct :`R` 1.0 :`B` 0.014634 :`A` 1.0) 20.0))
    (:`OnFailure`
      (`KismetSystemLibrary.PrintString` (`KismetStringLibrary.Concat_StrStr` "END PLAY REASON: " (`|GetEnumeratorNameAsString` EndPlayReason) " NO SESSION") true true (struct :`R` 1.0 :`B` 0.014634 :`A` 1.0) 20.0))))

(event `self.ReceiveTick`
  (params (DeltaSeconds :type "Float (single-precision)")))

(event `InputAction|LeftClick`
  (params (Key :type "Key Structure"))
  (bind _hitresult (`self.GetHitResultUnderCursorByChannel` (`GameplayStatics.GetPlayerController` 0) "TraceTypeQuery1" false))
  (:`Pressed`
    (bind _asworld_generator (cast `/Game/WorldGenerator` (`.HitActor` (`GameplayStatics.BreakHitResult` _hitresult))))
    (bind _asinstanced_static_mesh_component (cast `InstancedStaticMeshComponent` (`.HitComponent` (`GameplayStatics.BreakHitResult` _hitresult))))
    (bind _outinstancetransform (`InstancedStaticMeshComponent.GetInstanceTransform` _asinstanced_static_mesh_component (`.HitItem` (`GameplayStatics.BreakHitResult` _hitresult)) false))
    (`self.Request Place Creature` (`/Game/Blueprints/Utility/LIB_BP_General.2D to 1D index` (`/Game/WorldGenerator.HexWorldPosToIndex` _asworld_generator (`KismetMathLibrary.MakeVector2D` (.x (.location _outinstancetransform)) (.y (.location _outinstancetransform)))) (`/Game/WorldGenerator.MAX_Y` _asworld_generator)))))

(event `Request Place Creature`
  (params (Pos :type Integer))
  (bind _outactors (`GameplayStatics.GetAllActorsOfClass` "/Game/WorldGenerator.WorldGenerator_C"))
  (`/Game/WorldGenerator.Spawn Creature` _outactors Pos)
  (`KismetSystemLibrary.PrintString` "Hello"))

(event `InputAction|RightClick` :consume false
  (params (Key :type "Key Structure"))
  (bind _hitresult (`self.GetHitResultUnderCursorByChannel` (`GameplayStatics.GetPlayerController` 0) "TraceTypeQuery1" false))
  (:`Pressed`
    (bind _asworld_generator (cast `/Game/WorldGenerator` (`.HitActor` (`GameplayStatics.BreakHitResult` _hitresult))))
    (bind _asinstanced_static_mesh_component (cast `InstancedStaticMeshComponent` (`.HitComponent` (`GameplayStatics.BreakHitResult` _hitresult))))
    (bind _outinstancetransform (`InstancedStaticMeshComponent.GetInstanceTransform` _asinstanced_static_mesh_component (`.HitItem` (`GameplayStatics.BreakHitResult` _hitresult)) false))
    (`self.AltitudeChange(Server)` (`/Game/Blueprints/Utility/LIB_BP_General.2D to 1D index` (`/Game/WorldGenerator.HexWorldPosToIndex` _asworld_generator (`KismetMathLibrary.MakeVector2D` (.x (.location _outinstancetransform)) (.y (.location _outinstancetransform)))) (`/Game/WorldGenerator.MAX_Y` _asworld_generator)) -1.0)))

(event `AltitudeChange(Server)`
  (params (Index :type Integer) (Direction :type "Float (double-precision)"))
  (bind _values (`BlueprintMapLibrary.Map_Values` (`/Game/Blueprints/FFA/GM_FFA.ConnectedPlayers` (`/Game/Blueprints/Utility/LIB_BP_Casting.Get FFA Game Mode`))))
  (`self.AltitudeChange(Client)` _values Index Direction))

(event `AltitudeChange(Client)`
  (params (Index :type Integer) (Direction :type "Float (double-precision)"))
  (bind _outactors (`GameplayStatics.GetAllActorsOfClass` "/Game/WorldGenerator.WorldGenerator_C"))
  (`/Game/WorldGenerator.UpdateAltitude` _outactors Index Direction))

(fn `UserConstructionScript`)