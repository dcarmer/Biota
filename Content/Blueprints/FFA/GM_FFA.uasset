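; Game mode for free-for-all matches that tracks connected players and gives each one their own team.
; Post-login and controller swaps register the PC_FFA in a map keyed by PlayerId, with login also assigning a new team from the game state to PS_FFA.
; Logout removes the player and sends a "Left Game" feed entry to all remaining controllers.
; Login and swap also print debug messages on screen.
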(event `self.K2_OnSwapPlayerControllers`
  (params (OldPC :type "PlayerController Object Reference") (NewPC :type "PlayerController Object Reference"))
  (bind _aspc_ffa (cast `/Game/Blueprints/FFA/PC_FFA` NewPC :!pure true))
  (`BlueprintMapLibrary.Map_Add` (`self.ConnectedPlayers`) (`PlayerState.PlayerId` (`Controller.PlayerState` _aspc_ffa)) _aspc_ffa)
  (`KismetSystemLibrary.PrintString` (`KismetStringLibrary.Concat_StrStr` "SWAPPING PC TO: " (`KismetSystemLibrary.GetClassDisplayName` (`GameplayStatics.GetObjectClass` NewPC))) true true (struct :`R` 1.0 :`G` 0.065432 :`A` 1.0) 20.0))

(event `self.K2_PostLogin`
  (params (NewPlayer :type "PlayerController Object Reference"))
  (bind _aspc_ffa (cast `/Game/Blueprints/FFA/PC_FFA` NewPlayer :!pure true))
  (bind _playerstate (`Controller.PlayerState` _aspc_ffa))
  (`BlueprintMapLibrary.Map_Add` (`self.ConnectedPlayers`) (`PlayerState.PlayerId` _playerstate) _aspc_ffa)
  (bind _teamid (`/Game/Blueprints/FFA/GS_FFA.MakeNewTeam` (`/Game/Blueprints/Utility/LIB_BP_Casting.Get FFA Game State`)))
  (bind _output_get (set `/Game/Blueprints/FFA/PS_FFA.TeamId` _teamid (cast `/Game/Blueprints/FFA/PS_FFA` _playerstate :!pure true)))
  (`KismetSystemLibrary.PrintString` (`KismetStringLibrary.Concat_StrStr` "Login PC" " " (`KismetStringLibrary.Conv_IntToString` _output_get)) true true (struct :`R` 0.005958 :`G` 1.0 :`A` 1.0) 20.0))

(event `self.K2_OnLogout`
  (params (ExitingController :type "Controller Object Reference"))
  (bind _playerstate (`Controller.PlayerState` ExitingController))
  (bind _playerid (`PlayerState.PlayerId` _playerstate))
  (`BlueprintMapLibrary.Map_Remove` (`self.ConnectedPlayers`) _playerid)
  (bind _values (`BlueprintMapLibrary.Map_Values` (`self.ConnectedPlayers`)))
  (`/Game/Blueprints/FFA/PC_FFA.RecieveFeedEntry` _values (make `/Game/UI/NotificationFeed/S_GameMessage` "NewEnumerator3" _playerid (`|FormatText` "{Player} Left Game" (`KismetTextLibrary.Conv_StringToText` (`PlayerState.PlayerName` _playerstate))))))

(fn `UserConstructionScript`)