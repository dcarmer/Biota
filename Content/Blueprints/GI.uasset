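; Game Instance that manages multiplayer sessions, map travel and the loading screen.
; It hosts a listen-server lobby, joins or destroys sessions, server-travels to the game map and forwards name changes to the Game Mode.
; A loading widget created at Init shows during map loads.
; Network errors are stored, and an EndPlay binding on the player controller opens the error map, working around the forced default-map load.
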(event `StartGame`
  (`KismetSystemLibrary.ExecuteConsoleCommand` (`KismetStringLibrary.Concat_StrStr` "ServerTravel " (`KismetStringLibrary.Conv_NameToString` (`self.MAP_NAME_GAME`)))))

(event `HostGame`
  (params (`Player Controller` :type "PlayerController Object Reference") (PublicConnections :type Integer) (bUseLAN :type Boolean))
  (`CreateSessionCallbackProxy.CreateSession` `Player Controller` PublicConnections bUseLAN
    (:`OnSuccess`
      (`KismetSystemLibrary.PrintString` "STARTING SESSION")
      (set `self.PublicConnections` PublicConnections)
      (`GameplayStatics.OpenLevel` (`self.MAP_NAME_LOBBY`) true "listen"))
    (:`OnFailure`
      (`KismetSystemLibrary.PrintString` "Failed To Host Session"))))

(event `JoinGame`
  (params (`Player Controller` :type "PlayerController Object Reference") (Session :type "BlueprintSessionResult Structure"))
  (`JoinSessionCallbackProxy.JoinSession` `Player Controller` Session
    (:`OnFailure`
      (`KismetSystemLibrary.PrintString` "Failed To Join Session"))))

(event `LeaveGame`
  (params (`Player Controller` :type "PlayerController Object Reference"))
  (`DestroySessionCallbackProxy.DestroySession` `Player Controller`
    (:`OnSuccess`
      (`KismetSystemLibrary.PrintString` "Stopped Session"))
    (:`OnFailure`
      (`KismetSystemLibrary.PrintString` "Failed To Stop Session")))
  (`GameplayStatics.OpenLevel` (`self.MAP_NAME_START`)))

(event `self.HandleTravelError`
  (params (FailureType :type "ETravelFailure Enum" :default "NoLevel"))
  (`KismetSystemLibrary.PrintString` (`KismetStringLibrary.Concat_StrStr` "Travel Error: " (`|GetEnumeratorNameAsString` FailureType))))

(event `self.HandleNetworkError`
  (params (FailureType :type "ENetworkFailure Enum" :default "NetDriverAlreadyExists") (bIsServer :type Boolean))
  (`KismetSystemLibrary.PrintString` (`KismetStringLibrary.Concat_StrStr` "Network Error: " (`|GetEnumeratorNameAsString` FailureType) " Is Server: " (`KismetStringLibrary.Conv_BoolToString` bIsServer)))
  (set `self.NetworkError` FailureType)
  ;[1 0 0] Cause for whatever dumb reason, failure force loads default map, and cant be changed
  (add `Actor.OnEndPlay` (`GameplayStatics.GetPlayerController` 0) (delegate `Custom Event`)))

(event `Custom Event`
  (params (Actor :type "Actor Object Reference") (EndPlayReason :type "EEndPlayReason Enum" :default "Destroyed"))
  ;[1 0 0] Cause for whatever dumb reason, failure force loads default map, and cant be changed
  (`GameplayStatics.OpenLevel` (`self.MAP_NAME_NET_ERROR`))
  (remove `Actor.OnEndPlay` Actor (delegate `Custom Event`)))

(event `ChangeName`
  (params (Controller :type "Controller Object Reference") (NewName :type String))
  (`GameModeBase.ChangeName` (`GameplayStatics.GetGameMode`) Controller NewName true))

(event `self.ReceiveInit`
  (bind _returnvalue (`|CreateWidget` "/Game/UI/W_Loading.W_Loading_C" (`GameplayStatics.GetPlayerController` 0)))
  (set `self.W_Loading` _returnvalue))

(event `self.ReceiveShutdown`)

(event `self.OnPreLoadMap`
  (params (InMapName :type String))
  (bind _w_loading (`self.W_Loading`))
  (`/Engine/EditorBlueprintResources/StandardMacros.IsValid` _w_loading
    (:`Is Valid`
      (`UserWidget.AddToViewport` _w_loading 0))))

(event `self.OnPostLoadMapWithWorld`
  (params (InLoadedWorld :type "World Object Reference"))
  (bind _w_loading (`self.W_Loading`))
  (`/Engine/EditorBlueprintResources/StandardMacros.IsValid` _w_loading
    (:`Is Valid`
      (`Widget.RemoveFromParent` _w_loading))))