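; Hex-tile action object with an area footprint, a lifespan bar and helper functions for changing the world around it.
; On BeginPlay it polls until WorldGen is valid, caches tiles within its radius, marks each with a mesh instance and initializes the billboard timer.
; ApplyEffect functions modify creature nutrients or tile food, radiation, gather bonus and altitude, but are not called here.
; Altitude changes also move the tile instance, creature and action object at that position.
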(event `self.ReceiveBeginPlay`
  (bind _initiallifespan (`self.InitialLifeSpan`))
  (bind _worldgen (`/Game/Blueprints/FFA/GS_FFA.WorldGen` (`/Game/Blueprints/Utility/LIB_BP_Casting.Get FFA Game State`)))
  (`/Engine/EditorBlueprintResources/StandardMacros.IsValid` _worldgen :!label _label
    (:`Is Valid`
      (`|ExecutionSequence`
        (:`then_0`
          (bind _result (`/Game/WorldGenerator.GetValidNeighborsInRange` _worldgen (`self.Position`) (`self.RADIUS`)))
          (set `self.TilesUnderEffect` _result))
        (:`then_1`
          (for _array_element (`self.TilesUnderEffect`)
            (bind _transform (`/Game/WorldGenerator.GetTileTransform` _worldgen _array_element))
            (`InstancedStaticMeshComponent.AddInstanceWorldSpace` (`self.InstancedStaticMesh`) (`KismetMathLibrary.MakeTransform` (.location _transform) (struct) (`SceneComponent.K2_GetComponentScale` (`self.InstancedStaticMesh`))))))
        (:`then_2`
          (bind _astimer_bar (cast `/Game/UI/TimerBar` (`WidgetComponent.GetUserWidgetObject` (`self.WidgetBillboard`))))
          (set `/Game/UI/TimerBar.Initial` _initiallifespan _astimer_bar)
          (set `/Game/UI/TimerBar.Current` _initiallifespan _astimer_bar))))
    (:`Is Not Valid`
      (`KismetSystemLibrary.Delay` 0.2)
      (goto _label))))

(fn `ApplyEffect_AltitudeChange`
  (params (Position :type Integer) (Value :type "Float (double-precision)"))
  (locals (NewLocation :type "Vector Structure"))
  (bind _worldgen (`/Game/Blueprints/FFA/GS_FFA.WorldGen` (`/Game/Blueprints/Utility/LIB_BP_Casting.Get FFA Game State`)))
  (bind _output (`|GetArrayItem` (`/Game/WorldGenerator.HexTiles` _worldgen) Position))
  (bind _output_2 (`|GetArrayItem` (`/Game/WorldGenerator.Creature` _worldgen) Position))
  (bind _output_3 (`|GetArrayItem` (`/Game/WorldGenerator.ActionObjects` _worldgen) Position))
  (bind _outinstancetransform (`InstancedStaticMeshComponent.GetInstanceTransform` (break `/Game/S_ISMC_Ref` (`.ISMC_2_7520690A45C8AA80148792ABCB8AC5C4` (break `/Game/S_HexTile` _output))) (`.InstanceIndex_8_06E3E63440009B92B413C4A6D01EDE6C` (break `/Game/S_ISMC_Ref` (`.ISMC_2_7520690A45C8AA80148792ABCB8AC5C4` (break `/Game/S_HexTile` _output)))) false))
  (bind (_pos_x _pos_y) (`KismetMathLibrary.BreakVector2D` (`/Game/WorldGenerator.HexIndexToWorldPos` _worldgen (`/Game/Blueprints/Utility/LIB_BP_General.1D to 2D index` Position (`/Game/WorldGenerator.MAX_Y` _worldgen)))))
  (`|ExecutionSequence`
    (:`then_0`
      (`/Game/Blueprints/Utility/LIB_BP_General.+=(Float)` (break `/Game/S_HexTile` _output) Value)
      (bind _output_get (set `local.NewLocation` (`KismetMathLibrary.MakeVector` _pos_x _pos_y (break `/Game/S_HexTile` _output))))
      (`InstancedStaticMeshComponent.UpdateInstanceTransform` (break `/Game/S_ISMC_Ref` (`.ISMC_2_7520690A45C8AA80148792ABCB8AC5C4` (break `/Game/S_HexTile` _output))) (`.InstanceIndex_8_06E3E63440009B92B413C4A6D01EDE6C` (break `/Game/S_ISMC_Ref` (`.ISMC_2_7520690A45C8AA80148792ABCB8AC5C4` (break `/Game/S_HexTile` _output)))) (`KismetMathLibrary.MakeTransform` _output_get (.rotation _outinstancetransform) (.scale _outinstancetransform)) false true true))
    (:`then_1`
      (`/Engine/EditorBlueprintResources/StandardMacros.IsValid` _output_2
        (:`Is Valid`
          (`self.K2_SetActorLocation` _output_2 (`local.NewLocation`) false false))))
    (:`then_2`
      (`/Engine/EditorBlueprintResources/StandardMacros.IsValid` _output_3
        (:`Is Valid`
          (`self.K2_SetActorLocation` _output_3 (`local.NewLocation`) false false))))))

(fn `ApplyEffect_FoodChange`
  (params (Position :type Integer) (Value :type "Float (double-precision)"))
  (bind (_output_altitude _output_nutrientsavailable) (break `/Game/S_HexTile` (`|GetArrayItem` (`/Game/WorldGenerator.HexTiles` (`/Game/Blueprints/FFA/GS_FFA.WorldGen` (`/Game/Blueprints/Utility/LIB_BP_Casting.Get FFA Game State`))) Position)))
  (`|VariableSetRef` _output_nutrientsavailable (`KismetMathLibrary.FMax` (+ _output_nutrientsavailable Value))))

(fn `ApplyEffect_GatherBonusChange`
  (params (Position :type Integer) (Value :type "Float (double-precision)"))
  (bind (_output_altitude _output_nutrientsavailable _output_nutrientmax _output_nutrientgenerationrate _output_ismc _output_gatherratebonus) (break `/Game/S_HexTile` (`|GetArrayItem` (`/Game/WorldGenerator.HexTiles` (`/Game/Blueprints/FFA/GS_FFA.WorldGen` (`/Game/Blueprints/Utility/LIB_BP_Casting.Get FFA Game State`))) Position)))
  (`/Game/Blueprints/Utility/LIB_BP_General.+=(Float)` _output_gatherratebonus Value))

(fn `ApplyEffect_HealthChange`
  (params (Position :type Integer) (Value :type "Float (double-precision)"))
  (bind _output (`|GetArrayItem` (`/Game/WorldGenerator.Creature` (`/Game/Blueprints/FFA/GS_FFA.WorldGen` (`/Game/Blueprints/Utility/LIB_BP_Casting.Get FFA Game State`))) Position))
  (`/Engine/EditorBlueprintResources/StandardMacros.IsValid` _output
    (:`Is Valid`
      (`/Game/Blueprints/Utility/LIB_BP_General.+=(Float)` (`/Game/Creature.StoredNutrients` _output) Value))))

(fn `ApplyEffect_RadiationChange`
  (params (Position :type Integer) (Value :type "Float (double-precision)"))
  (bind (_output_altitude _output_nutrientsavailable _output_nutrientmax _output_nutrientgenerationrate _output_ismc _output_gatherratebonus _output_radioactivity) (break `/Game/S_HexTile` (`|GetArrayItem` (`/Game/WorldGenerator.HexTiles` (`/Game/Blueprints/FFA/GS_FFA.WorldGen` (`/Game/Blueprints/Utility/LIB_BP_Casting.Get FFA Game State`))) Position)))
  (`|VariableSetRef` _output_radioactivity (`KismetMathLibrary.FMax` (+ _output_radioactivity Value))))

(fn `UserConstructionScript`)